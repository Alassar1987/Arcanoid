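; BP_Ball is the Arcanoid ball, bouncing around in the XZ plane until it is lost.
; Tick moves it by a swept offset of Direction times Velocity, unscaled by delta time, and reflects Direction off blocking surface normals.
; Hit events multiply Velocity up to a clamp.
; Overlapping a KillZVolume calls BallLost, then destroys the ball shortly after; the rotate-to-direction function is never executed.
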(event `self.ReceiveActorBeginOverlap`
  (params (OtherActor :type "Actor Object Reference"))
  ;[1 1 1] Lossing Ball logic
  (castclass `KillZVolume` (`GameplayStatics.GetObjectClass` OtherActor))
  (`self.BallLost`)
  (`KismetSystemLibrary.Delay` 0.05)
  (`self.K2_DestroyActor`))

(event `self.ReceiveBeginPlay`
  ;[1 1 1] Rotate ball forward to moving direction
)

(event `self.ReceiveHit`
  (params (MyComp :type "PrimitiveComponent Object Reference") (Other :type "Actor Object Reference") (OtherComp :type "PrimitiveComponent Object Reference") (bSelfMoved :type Boolean) (HitLocation :type "Vector Structure") (HitNormal :type "Vector Structure") (NormalImpulse :type "Vector Structure") (Hit :type "HitResult Structure (by ref)"))
  ;[1 1 1] Velocity changing on hit
  (set `self.Velocity` (`KismetMathLibrary.FClamp` (* (`self.Velocity`) (`self.VelocityMultiplier`)) 0.0 25.0)))

(event `self.ReceiveTick`
  (params (DeltaSeconds :type "Float (single-precision)"))
  ;[1 1 1] Moving logic
  (bind _sweephitresult (`self.K2_AddActorWorldOffset` (`KismetMathLibrary.MakeVector` (.x (* (`self.Direction`) (`self.Velocity`))) 0.0 (.z (* (`self.Direction`) (`self.Velocity`)))) true))
  (bind (_bblockinghit _binitialoverlap _time _distance _location _impactpoint _normal) (`GameplayStatics.BreakHitResult` _sweephitresult))
  (if _bblockinghit
    (set `self.Direction` (`KismetMathLibrary.GetReflectionVector` (`self.Direction`) _normal))
    (`KismetSystemLibrary.Delay` 0.01)))

(fn `F_RotationUpdate`
  ;[1 1 1] Rotate Ball according to hit
  (`self.K2_AddActorWorldRotation` (`KismetMathLibrary.Conv_VectorToRotator` (`self.Direction`))))

(fn `UserConstructionScript`)