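; Moving projectile actor for the Arcanoid game that bounces off blocking surfaces and changes speed on each hit.
; Tick moves it by Direction times Velocity with a swept offset, unscaled by delta time, and reflects Direction about the hit normal.
; Hit events scale Velocity by a multiplier, clamp it and print it.
; BeginPlay and Hit also add a local rotation derived from Direction.
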(event `self.ReceiveBeginPlay`
  (`self.F_RotationUpdate`))

(event `self.ReceiveHit`
  (params (MyComp :type "PrimitiveComponent Object Reference") (Other :type "Actor Object Reference") (OtherComp :type "PrimitiveComponent Object Reference") (bSelfMoved :type Boolean) (HitLocation :type "Vector Structure") (HitNormal :type "Vector Structure") (NormalImpulse :type "Vector Structure") (Hit :type "HitResult Structure (by ref)"))
  (`self.F_RotationUpdate`)
  (bind _output_get (set `self.Velocity` (`KismetMathLibrary.FClamp` (* (`self.Velocity`) (`self.VelocityMultiplier`)) 0.0 25.0)))
  (`KismetSystemLibrary.PrintString` (`KismetStringLibrary.Conv_DoubleToString` _output_get) true true (struct :`G` 0.66 :`B` 1.0 :`A` 1.0) 3.0))

(event `self.ReceiveTick`
  (params (DeltaSeconds :type "Float (single-precision)"))
  (bind _sweephitresult (`self.K2_AddActorWorldOffset` (* (`self.Direction`) (`self.Velocity`)) true))
  (bind (_bblockinghit _binitialoverlap _time _distance _location _impactpoint _normal) (`GameplayStatics.BreakHitResult` _sweephitresult))
  (if _bblockinghit
    (set `self.Direction` (`KismetMathLibrary.GetReflectionVector` (`self.Direction`) _normal))))

(fn `F_RotationUpdate`
  (`self.K2_AddActorLocalRotation` (`KismetMathLibrary.Conv_VectorToRotator` (`self.Direction`))))

(fn `UserConstructionScript`)